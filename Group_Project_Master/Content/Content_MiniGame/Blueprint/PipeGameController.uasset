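; Player controller for the pipe minigame that turns mouse and keyboard input into calls on the map reference.
; A left click deprojects the cursor and traces along negative Y on the Visibility channel, with debug drawing.
; On a hit it stores the deprojected cursor position, not the impact point, as the game mode's HitLocation, then calls SwitchTile.
; Space bar forwards to the map's SpaceBarPressed, while mouse release does nothing beyond a game mode cast.
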(event `Key|LeftMouseButton`
  (params (Key :type "Key Structure" :default "AnyKey"))
  (bind _worldlocation (`self.DeprojectMousePositionToWorld`))
  (:`Pressed`
    (bind (_outhit _returnvalue) (`KismetSystemLibrary.LineTraceSingle` :`Start` _worldlocation :`End` (- _worldlocation (0.0 1000.0 0.0)) :`TraceChannel` "TraceTypeQuery1" :`DrawDebugType` "ForDuration"))
    (if _returnvalue
      (bind _asgm_pipe_game (cast `/Game/Content_MiniGame/Blueprint/GameModes/GM_Pipe_game` (`GameplayStatics.GetGameMode`)))
      (set `/Game/Content_MiniGame/Blueprint/GameModes/GM_Pipe_game.Hit location` _worldlocation _asgm_pipe_game)
      (`/Game/Content_MiniGame/Blueprint/BP_TileMap_Pipe.SwitchTile` (`self.map_ref`))
      (else
        (cast `/Game/Content_MiniGame/Blueprint/GameModes/GM_Pipe_game` (`GameplayStatics.GetGameMode`) :!label _label))))
  (:`Released`
    (goto _label)))

(event `Key|SpaceBar`
  (params (Key :type "Key Structure" :default "AnyKey"))
  (:`Pressed`
    (`/Game/Content_MiniGame/Blueprint/BP_TileMap_Pipe.SpaceBarPressed` (`self.map_ref`))))

(fn `UserConstructionScript`)