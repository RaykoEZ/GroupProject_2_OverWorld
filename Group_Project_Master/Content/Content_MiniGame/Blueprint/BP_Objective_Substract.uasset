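; Minigame objective that lowers the player's Count when an actor overlaps it.
; On BeginPlay it registers with the game mode and sets Completed to true.
; Each overlap, with no check on the overlapping actor, tints the FLIPDummy sprite dark red, decrements BP_PlayerChar's Count and prints.
; Completed stays true, so the green increment branch is not reached within this Blueprint, and the objective-cleared call is disconnected.
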(event `self.ReceiveBeginPlay`
  ;[1 1 1] Get Existing Objectives
  (`/Game/Content_MiniGame/Blueprint/BPI_NodeCleared.registerObjective`)
  (set `self.Completed` true))

(event `/Game/Content_MiniGame/Blueprint/BPI_NodeCleared.registerObjective`
  ;[1 1 1] Get Existing Objectives
  (message `/Game/Content_MiniGame/Blueprint/BPI_NodeCleared.registerObjective` (`GameplayStatics.GetGameMode`)))

(event `self.ReceiveActorBeginOverlap`
  (params (OtherActor :type "Actor Object Reference"))
  ;[1 1 1] When an objective is reached
  (if (`self.Completed`)
    (`PaperFlipbookComponent.SetSpriteColor` (`self.FLIP_Dummy`) (`KismetMathLibrary.MakeColor` 0.2 0.0 0.0))
    (bind _asbp_player_char (cast `/Game/Content_MiniGame/Blueprint/BP_PlayerChar` (`GameplayStatics.GetPlayerCharacter` 0)))
    (bind _returnvalue (+ (`/Game/Content_MiniGame/Blueprint/BP_PlayerChar.Count` _asbp_player_char) -1))
    (set `/Game/Content_MiniGame/Blueprint/BP_PlayerChar.Count` _returnvalue _asbp_player_char)
    (set `self.Completed` true)
    (`KismetSystemLibrary.PrintString` (`KismetStringLibrary.Conv_IntToString` _returnvalue))
    (else
      (`PaperFlipbookComponent.SetSpriteColor` (`self.FLIP_Dummy`) (`KismetMathLibrary.MakeColor` 0.0 1.0 0.2))
      (bind _asbp_player_char_2 (cast `/Game/Content_MiniGame/Blueprint/BP_PlayerChar` (`GameplayStatics.GetPlayerCharacter` 0)))
      (bind _returnvalue_2 (+ (`/Game/Content_MiniGame/Blueprint/BP_PlayerChar.Count` _asbp_player_char_2) 1))
      (set `/Game/Content_MiniGame/Blueprint/BP_PlayerChar.Count` _returnvalue_2 _asbp_player_char_2)
      (set `self.Completed` false)
      (`KismetSystemLibrary.PrintString` (`KismetStringLibrary.Conv_IntToString` _returnvalue_2)))))

(fn `UserConstructionScript`)