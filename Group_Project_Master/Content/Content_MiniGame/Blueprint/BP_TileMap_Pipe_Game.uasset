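; Paper2D tile map actor for a pipe mini-game that switches the pipe tile at a hit location.
; SwitchTile reads HitLocation from GM_Pipe_game, converts its offset from Origin into 64-unit grid coordinates, then looks up that tile's TileTypes index.
; SolveTileType steps the index through a four-state cycle or a two-state toggle before the tile is rewritten.
; Unmatched tiles receive the first TileTypes entry.
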(event `SwitchTile`
  (bind (_returnvalue _returnvalue2) (`self.GetTilePos`))
  (set `self.Tile_Num` 0)
  (`PaperTileMapComponent.MakeTileMapEditable` (`self.PaperTileMap`))
  (`self.CheckTilePos`)
  (`self.SolveTileType`)
  (`PaperTileMapComponent.SetTile` (`self.PaperTileMap`) _returnvalue _returnvalue2 0 (`|GetArrayItem` (`self.TileTypes`) (`self.Tile_Num`))))

(fn `CheckTilePos`
  (bind _asgm_pipe_game (cast `/Game/Content_MiniGame/Blueprint/GameModes/GM_Pipe_game` (`GameplayStatics.GetGameMode`)))
  (set `self.HitLocation` (`/Game/Content_MiniGame/Blueprint/GameModes/GM_Pipe_game.Hit location` _asgm_pipe_game)))

(fn `PrintTilePos`
  (bind (_returnvalue _returnvalue2) (`self.GetTilePos`))
  (`KismetSystemLibrary.PrintString` (`KismetStringLibrary.Conv_VectorToString` (`KismetMathLibrary.MakeVector` (`KismetMathLibrary.Conv_IntToDouble` _returnvalue) 0.0 (`KismetMathLibrary.Conv_IntToDouble` _returnvalue2)))))

(fn `SolveTileType`
  (if (== (`self.GetTileType`) 9)
    (set `self.Tile_Num` 10)
    (elif (== (`self.GetTileType`) 10)
      (set `self.Tile_Num` 8)
      (elif (== (`self.GetTileType`) 8)
        (set `self.Tile_Num` 7)
        (elif (== (`self.GetTileType`) 7)
          (set `self.Tile_Num` 9)
          (elif (== (`self.GetTileType`) 12)
            (set `self.Tile_Num` 13)
            (elif (== (`self.GetTileType`) 13)
              (set `self.Tile_Num` 12))))))))

(fn `UserConstructionScript`
  (`PaperTileMapComponent.SetTileMap` (`self.PaperTileMap`) (`self.Map`)))