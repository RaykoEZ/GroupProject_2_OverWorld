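; Minigame objective that acts as a toggleable math operator on the player's Count, registering with the GameMode at BeginPlay.
; When an overlap ends, OperatorType selects add, subtract or multiply by the player's SavedNumber.
; The Completed flag alternates between applying and reversing the operation, swapping red and yellow flipbooks and printing debug text.
; ModulusOperator is never called, and the objective-cleared notification is disconnected.
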(event `self.ReceiveBeginPlay`
  ;[1 1 1] Get Existing Objectives
  (`/Game/Content_MiniGame/Blueprint/BPI_NodeCleared.registerObjective`)
  (set `self.Completed` true))

(event `/Game/Content_MiniGame/Blueprint/BPI_NodeCleared.registerObjective`
  ;[1 1 1] Get Existing Objectives
  (message `/Game/Content_MiniGame/Blueprint/BPI_NodeCleared.registerObjective` (`GameplayStatics.GetGameMode`)))

(event `self.ReceiveActorBeginOverlap`
  (params (OtherActor :type "Actor Object Reference"))
  ;[1 1 1] When an objective is reached
)

(event `self.ReceiveActorEndOverlap`
  (params (OtherActor :type "Actor Object Reference"))
  ;[1 1 1] When an objective is reached
  (switch `/Engine/ArtTools/RenderToTexture/Enums/EIntTypes` (`self.OperatorType`)
    (:`NewEnumerator4`
      (`self.Add_Operator`))
    (:`NewEnumerator5`
      (`self.Substract_Operator`))
    (:`NewEnumerator6`
      (`self.Multiply_Operator`))))

(fn `Add_Operator`
  (if (`self.Completed`)
    (`PaperFlipbookComponent.SetFlipbook` (`self.FLIP_Dummy`) "/Game/Content_MiniGame/Sprite/Flipbooks/FB_Red.FB_Red")
    (bind _asbp_player_char (cast `/Game/Content_MiniGame/Blueprint/BP_PlayerChar` (`GameplayStatics.GetPlayerCharacter` 0)))
    (bind _returnvalue (+ (`/Game/Content_MiniGame/Blueprint/BP_PlayerChar.Count` _asbp_player_char) (`/Game/Content_MiniGame/Blueprint/BP_PlayerChar.Saved_Number` _asbp_player_char)))
    (set `/Game/Content_MiniGame/Blueprint/BP_PlayerChar.Count` _returnvalue _asbp_player_char)
    (set `self.Completed` false)
    (`KismetSystemLibrary.PrintString` (`KismetStringLibrary.Conv_IntToString` _returnvalue))
    (else
      (`PaperFlipbookComponent.SetFlipbook` (`self.FLIP_Dummy`) "/Game/Content_MiniGame/Sprite/Flipbooks/FB_Yellow.FB_Yellow")
      (bind _asbp_player_char_2 (cast `/Game/Content_MiniGame/Blueprint/BP_PlayerChar` (`GameplayStatics.GetPlayerCharacter` 0)))
      (bind _returnvalue_2 (- (`/Game/Content_MiniGame/Blueprint/BP_PlayerChar.Count` _asbp_player_char_2) (`/Game/Content_MiniGame/Blueprint/BP_PlayerChar.Saved_Number` _asbp_player_char_2)))
      (set `/Game/Content_MiniGame/Blueprint/BP_PlayerChar.Count` _returnvalue_2 _asbp_player_char_2)
      (set `self.Completed` true)
      (`KismetSystemLibrary.PrintString` (`KismetStringLibrary.Conv_IntToString` _returnvalue_2)))))

(fn `Modulus_Operator`
  (if (`self.Completed`)
    (`PaperFlipbookComponent.SetFlipbook` (`self.FLIP_Dummy`) "/Game/Content_MiniGame/Sprite/Flipbooks/FB_Red.FB_Red")
    (bind _asbp_player_char (cast `/Game/Content_MiniGame/Blueprint/BP_PlayerChar` (`GameplayStatics.GetPlayerCharacter` 0)))
    (bind _returnvalue (mod (`/Game/Content_MiniGame/Blueprint/BP_PlayerChar.Count` _asbp_player_char) (`/Game/Content_MiniGame/Blueprint/BP_PlayerChar.Saved_Number` _asbp_player_char)))
    (set `/Game/Content_MiniGame/Blueprint/BP_PlayerChar.Count` _returnvalue _asbp_player_char)
    (set `self.Completed` false)
    (`KismetSystemLibrary.PrintString` (`KismetStringLibrary.Conv_IntToString` _returnvalue))
    (else
      (`PaperFlipbookComponent.SetFlipbook` (`self.FLIP_Dummy`) "/Game/Content_MiniGame/Sprite/Flipbooks/FB_Yellow.FB_Yellow")
      (bind _asbp_player_char_2 (cast `/Game/Content_MiniGame/Blueprint/BP_PlayerChar` (`GameplayStatics.GetPlayerCharacter` 0)))
      (bind _returnvalue_2 (`KismetMathLibrary.Round` (* (`KismetMathLibrary.Conv_IntToDouble` (`/Game/Content_MiniGame/Blueprint/BP_PlayerChar.Count` _asbp_player_char_2)) 0.5)))
      (set `/Game/Content_MiniGame/Blueprint/BP_PlayerChar.Count` _returnvalue_2 _asbp_player_char_2)
      (set `self.Completed` true)
      (`KismetSystemLibrary.PrintString` (`KismetStringLibrary.Conv_IntToString` _returnvalue_2)))))

(fn `Multiply_Operator`
  (if (`self.Completed`)
    (`PaperFlipbookComponent.SetFlipbook` (`self.FLIP_Dummy`) "/Game/Content_MiniGame/Sprite/Flipbooks/FB_Red.FB_Red")
    (bind _asbp_player_char (cast `/Game/Content_MiniGame/Blueprint/BP_PlayerChar` (`GameplayStatics.GetPlayerCharacter` 0)))
    (bind _returnvalue (* (`/Game/Content_MiniGame/Blueprint/BP_PlayerChar.Count` _asbp_player_char) (`/Game/Content_MiniGame/Blueprint/BP_PlayerChar.Saved_Number` _asbp_player_char)))
    (set `/Game/Content_MiniGame/Blueprint/BP_PlayerChar.Count` _returnvalue _asbp_player_char)
    (set `self.Completed` false)
    (`KismetSystemLibrary.PrintString` (`KismetStringLibrary.Conv_IntToString` _returnvalue))
    (else
      (`PaperFlipbookComponent.SetFlipbook` (`self.FLIP_Dummy`) "/Game/Content_MiniGame/Sprite/Flipbooks/FB_Yellow.FB_Yellow")
      (bind _asbp_player_char_2 (cast `/Game/Content_MiniGame/Blueprint/BP_PlayerChar` (`GameplayStatics.GetPlayerCharacter` 0)))
      (bind _returnvalue_2 (`KismetMathLibrary.Round` (/ (`KismetMathLibrary.Conv_IntToDouble` (`/Game/Content_MiniGame/Blueprint/BP_PlayerChar.Count` _asbp_player_char_2)) (`KismetMathLibrary.Conv_IntToDouble` (`/Game/Content_MiniGame/Blueprint/BP_PlayerChar.Saved_Number` _asbp_player_char_2)))))
      (set `/Game/Content_MiniGame/Blueprint/BP_PlayerChar.Count` _returnvalue_2 _asbp_player_char_2)
      (set `self.Completed` true)
      (`KismetSystemLibrary.PrintString` (`KismetStringLibrary.Conv_IntToString` _returnvalue_2)))))

(fn `Substract_Operator`
  (if (`self.Completed`)
    (`PaperFlipbookComponent.SetFlipbook` (`self.FLIP_Dummy`) "/Game/Content_MiniGame/Sprite/Flipbooks/FB_Red.FB_Red")
    (bind _asbp_player_char (cast `/Game/Content_MiniGame/Blueprint/BP_PlayerChar` (`GameplayStatics.GetPlayerCharacter` 0)))
    (bind _returnvalue (- (`/Game/Content_MiniGame/Blueprint/BP_PlayerChar.Count` _asbp_player_char) (`/Game/Content_MiniGame/Blueprint/BP_PlayerChar.Saved_Number` _asbp_player_char)))
    (set `/Game/Content_MiniGame/Blueprint/BP_PlayerChar.Count` _returnvalue _asbp_player_char)
    (set `self.Completed` false)
    (`KismetSystemLibrary.PrintString` (`KismetStringLibrary.Conv_IntToString` _returnvalue))
    (else
      (`PaperFlipbookComponent.SetFlipbook` (`self.FLIP_Dummy`) "/Game/Content_MiniGame/Sprite/Flipbooks/FB_Yellow.FB_Yellow")
      (bind _asbp_player_char_2 (cast `/Game/Content_MiniGame/Blueprint/BP_PlayerChar` (`GameplayStatics.GetPlayerCharacter` 0)))
      (bind _returnvalue_2 (+ (`/Game/Content_MiniGame/Blueprint/BP_PlayerChar.Count` _asbp_player_char_2) (`/Game/Content_MiniGame/Blueprint/BP_PlayerChar.Saved_Number` _asbp_player_char_2)))
      (set `/Game/Content_MiniGame/Blueprint/BP_PlayerChar.Count` _returnvalue_2 _asbp_player_char_2)
      (set `self.Completed` true)
      (`KismetSystemLibrary.PrintString` (`KismetStringLibrary.Conv_IntToString` _returnvalue_2)))))

(fn `UserConstructionScript`
  (switch `/Engine/ArtTools/RenderToTexture/Enums/EIntTypes` (`self.OperatorType`)
    (:`NewEnumerator4`
      (`PaperFlipbookComponent.SetFlipbook` (`self.FLIP_Dummy`) "/Game/Content_MiniGame/Sprite/Flipbooks/FB_Red.FB_Red"))
    (:`NewEnumerator5`
      (`PaperFlipbookComponent.SetFlipbook` (`self.FLIP_Dummy`) "/Game/Content_MiniGame/Sprite/Flipbooks/FB_Red.FB_Red"))
    (:`NewEnumerator6`
      (`PaperFlipbookComponent.SetFlipbook` (`self.FLIP_Dummy`) "/Game/Content_MiniGame/Sprite/Flipbooks/FB_Red.FB_Red"))
    (:`NewEnumerator7`
      (`PaperFlipbookComponent.SetFlipbook` (`self.FLIP_Dummy`) "/Game/Content_MiniGame/Sprite/Flipbooks/FB_Red.FB_Red"))))