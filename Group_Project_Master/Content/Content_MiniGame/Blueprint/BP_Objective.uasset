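; BP_Objective is a minigame objective marker that counts as cleared when an actor overlaps it.
; On BeginPlay it registers itself with the game mode through a message call.
; The first overlap tints its flipbook dummy sprite green, notifies the game mode that the objective is cleared, and sets a Completed flag so it only fires once.
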(event `self.ReceiveBeginPlay`
  ;[1 1 1] Get Existing Objectives
  (`/Game/Content_MiniGame/Blueprint/BPI_NodeCleared.registerObjective`))

(event `/Game/Content_MiniGame/Blueprint/BPI_NodeCleared.registerObjective`
  ;[1 1 1] Get Existing Objectives
  (message `/Game/Content_MiniGame/Blueprint/BPI_NodeCleared.registerObjective` (`GameplayStatics.GetGameMode`)))

(event `self.ReceiveActorBeginOverlap`
  (params (OtherActor :type "Actor Object Reference"))
  ;[1 1 1] When an objective is reached
  (if (== (`self.Completed`) false)
    (`PaperFlipbookComponent.SetSpriteColor` (`self.FLIP_Dummy`) (`KismetMathLibrary.MakeColor` 0.0 1.0 0.2))
    (message `/Game/Content_MiniGame/Blueprint/BPI_NodeCleared.objectiveCleared` (`GameplayStatics.GetGameMode`))
    (set `self.Completed` true)))

(fn `UserConstructionScript`)