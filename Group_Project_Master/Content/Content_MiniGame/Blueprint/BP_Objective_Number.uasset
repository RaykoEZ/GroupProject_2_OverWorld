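; Numbered objective actor for the minigame that hands its value to the game mode when an overlapping actor leaves it.
; The construction script picks its flipbook icon from ObjVal, and BeginPlay registers it with the game mode through a message call.
; The first end overlap writes ObjVal to GM_Test's PrevOperand, greys the icon, marks it completed and beeps.
; Later overlaps only play an error sound.
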(event `self.ReceiveBeginPlay`
  ;[1 1 1] Get Existing Objectives
  (`/Game/Content_MiniGame/Blueprint/BPI_NodeCleared.registerObjective`))

(event `/Game/Content_MiniGame/Blueprint/BPI_NodeCleared.registerObjective`
  ;[1 1 1] Get Existing Objectives
  (message `/Game/Content_MiniGame/Blueprint/BPI_NodeCleared.registerObjective` (`GameplayStatics.GetGameMode`)))

(event `self.ReceiveActorEndOverlap`
  (params (OtherActor :type "Actor Object Reference"))
  ;[1 1 1] When an objective is reached
  (if (`self.Completed`)
    (`/Game/Blueprints/BP_GeneralAudio.ErrorSound`)
    (else
      (bind _asgm_test (cast `/Game/Content_MiniGame/Blueprint/GameModes/GM_Test` (`GameplayStatics.GetGameMode`)))
      (set `/Game/Content_MiniGame/Blueprint/GameModes/GM_Test.PrevOperand` (`self.objVal`) _asgm_test)
      (`PaperFlipbookComponent.SetFlipbook` (`self.FLIP_Dummy`) (`|GetArrayItem` (`self.Grey_Icon`) (`self.objVal`)))
      (set `self.Completed` true)
      (`/Game/Blueprints/BP_GeneralAudio.Beep`))))

(fn `UserConstructionScript`
  (`PaperFlipbookComponent.SetFlipbook` (`self.FLIP_Dummy`) (`|GetArrayItem` (`self.Icons`) (`self.objVal`))))