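; Operator objective for a math minigame that applies an arithmetic operation to the score in GM_Test and registers with it on BeginPlay.
; The construction script picks a flipbook from OperatorType for add, subtract, multiply or modulus.
; Ending an overlap combines CurrentScore with PrevOperand's value once, then switches the flipbook and marks it Completed.
; Modulus has a function, but the overlap event never calls it.
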(event `self.ReceiveBeginPlay`
  ;[1 1 1] Get Existing Objectives
  (`/Game/Content_MiniGame/Blueprint/BPI_NodeCleared.registerObjective`))

(event `/Game/Content_MiniGame/Blueprint/BPI_NodeCleared.registerObjective`
  ;[1 1 1] Get Existing Objectives
  (message `/Game/Content_MiniGame/Blueprint/BPI_NodeCleared.registerObjective` (`GameplayStatics.GetGameMode`)))

(event `self.ReceiveActorBeginOverlap`
  (params (OtherActor :type "Actor Object Reference"))
  ;[1 1 1] When an objective is reached
)

(event `self.ReceiveActorEndOverlap`
  (params (OtherActor :type "Actor Object Reference"))
  ;[1 1 1] When an objective is reached
  (switch `/Engine/ArtTools/RenderToTexture/Enums/EIntTypes` (`self.OperatorType`)
    (:`NewEnumerator4`
      (`self.Add_Operator`))
    (:`NewEnumerator5`
      (`self.Substract_Operator`))
    (:`NewEnumerator6`
      (`self.Multiply_Operator`))))

(fn `Add_Operator`
  (if (not (`self.Completed`))
    (bind _gamomode (`self.getGameMode`))
    (bind _prevoperand (`/Game/Content_MiniGame/Blueprint/GameModes/GM_Test.PrevOperand` _gamomode))
    (`/Engine/EditorBlueprintResources/StandardMacros.IsValid` _prevoperand
      (:`Is Valid`
        (`PaperFlipbookComponent.SetFlipbook` (`self.FLIP_Dummy`) "/Game/Content_MiniGame/Sprite/Flipbooks/OpNumFlipbooks/F_OP_G_Add.F_OP_G_Add")
        (bind _returnvalue (+ (`/Game/Content_MiniGame/Blueprint/BP_Objective_Number.objVal` _prevoperand) (`/Game/Content_MiniGame/Blueprint/GameModes/GM_Test.CurrentScore` _gamomode)))
        (`self.UpdateGameMode` _returnvalue)
        (`KismetSystemLibrary.PrintString` (`KismetStringLibrary.Conv_IntToString` _returnvalue))
        (`KismetSystemLibrary.PrintString` "Added")
        (set `self.Completed` true)))))

(fn `getGameMode`
  (returns (GamoMode :type "/Game/Content_MiniGame/Blueprint/GameModes/GM_Test Object Reference"))
  (bind _asgm_test (cast `/Game/Content_MiniGame/Blueprint/GameModes/GM_Test` (`GameplayStatics.GetGameMode`)))
  (return _asgm_test))

(fn `Modulus_Operator`
  (if (not (`self.Completed`))
    (bind _gamomode (`self.getGameMode`))
    (`/Engine/EditorBlueprintResources/StandardMacros.IsValid` (`/Game/Content_MiniGame/Blueprint/GameModes/GM_Test.PrevOperand` _gamomode)
      (:`Is Valid`
        (bind _gamomode_2 (`self.getGameMode`))
        (bind _prevoperand (`/Game/Content_MiniGame/Blueprint/GameModes/GM_Test.PrevOperand` _gamomode_2))
        (`/Engine/EditorBlueprintResources/StandardMacros.IsValid` _prevoperand
          (:`Is Valid`
            (`PaperFlipbookComponent.SetFlipbook` (`self.FLIP_Dummy`) "/Game/Content_MiniGame/Sprite/Flipbooks/OpNumFlipbooks/F_OP_G_Mod.F_OP_G_Mod")
            (bind _returnvalue (mod (`/Game/Content_MiniGame/Blueprint/GameModes/GM_Test.CurrentScore` _gamomode_2) (`/Game/Content_MiniGame/Blueprint/BP_Objective_Number.objVal` _prevoperand)))
            (`self.UpdateGameMode` _returnvalue)
            (`KismetSystemLibrary.PrintString` (`KismetStringLibrary.Conv_IntToString` _returnvalue))
            (`KismetSystemLibrary.PrintString` "Added")
            (set `self.Completed` true)))))))

(fn `Multiply_Operator`
  (if (not (`self.Completed`))
    (bind _gamomode (`self.getGameMode`))
    (bind _prevoperand (`/Game/Content_MiniGame/Blueprint/GameModes/GM_Test.PrevOperand` _gamomode))
    (`/Engine/EditorBlueprintResources/StandardMacros.IsValid` _prevoperand
      (:`Is Valid`
        (`PaperFlipbookComponent.SetFlipbook` (`self.FLIP_Dummy`) "/Game/Content_MiniGame/Sprite/Flipbooks/OpNumFlipbooks/F_OP_G_Multiply.F_OP_G_Multiply")
        (bind _returnvalue (* (`/Game/Content_MiniGame/Blueprint/BP_Objective_Number.objVal` _prevoperand) (`/Game/Content_MiniGame/Blueprint/GameModes/GM_Test.CurrentScore` _gamomode)))
        (`self.UpdateGameMode` _returnvalue)
        (`KismetSystemLibrary.PrintString` (`KismetStringLibrary.Conv_IntToString` _returnvalue))
        (`KismetSystemLibrary.PrintString` "Added")
        (set `self.Completed` true)))))

(fn `Substract_Operator`
  (if (not (`self.Completed`))
    (bind _gamomode (`self.getGameMode`))
    (bind _prevoperand (`/Game/Content_MiniGame/Blueprint/GameModes/GM_Test.PrevOperand` _gamomode))
    (`/Engine/EditorBlueprintResources/StandardMacros.IsValid` _prevoperand
      (:`Is Valid`
        (`PaperFlipbookComponent.SetFlipbook` (`self.FLIP_Dummy`) "/Game/Content_MiniGame/Sprite/Flipbooks/OpNumFlipbooks/F_OP_G_Substract.F_OP_G_Substract")
        (bind _returnvalue (- (`/Game/Content_MiniGame/Blueprint/GameModes/GM_Test.CurrentScore` _gamomode) (`/Game/Content_MiniGame/Blueprint/BP_Objective_Number.objVal` _prevoperand)))
        (`self.UpdateGameMode` _returnvalue)
        (`KismetSystemLibrary.PrintString` (`KismetStringLibrary.Conv_IntToString` _returnvalue))
        (`KismetSystemLibrary.PrintString` "Added")
        (set `self.Completed` true)))))

(fn `UserConstructionScript`
  (switch `/Engine/ArtTools/RenderToTexture/Enums/EIntTypes` (`self.OperatorType`)
    (:`NewEnumerator4`
      (`PaperFlipbookComponent.SetFlipbook` (`self.FLIP_Dummy`) "/Game/Content_MiniGame/Sprite/Flipbooks/OpNumFlipbooks/F_OP_Add.F_OP_Add"))
    (:`NewEnumerator5`
      (`PaperFlipbookComponent.SetFlipbook` (`self.FLIP_Dummy`) "/Game/Content_MiniGame/Sprite/Flipbooks/OpNumFlipbooks/F_OP_Substract.F_OP_Substract"))
    (:`NewEnumerator6`
      (`PaperFlipbookComponent.SetFlipbook` (`self.FLIP_Dummy`) "/Game/Content_MiniGame/Sprite/Flipbooks/OpNumFlipbooks/F_OP_Multiply.F_OP_Multiply"))
    (:`NewEnumerator7`
      (`PaperFlipbookComponent.SetFlipbook` (`self.FLIP_Dummy`) "/Game/Content_MiniGame/Sprite/Flipbooks/OpNumFlipbooks/F_OP_Mod.F_OP_Mod"))))