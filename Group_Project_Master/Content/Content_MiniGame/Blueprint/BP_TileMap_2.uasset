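; BP_TileMap_2 is a Paper2D tile map actor for a minigame, with a SwitchTile event that changes the tile at a hit location.
; GetTilePos turns the offset between an Origin component and HitLocation into X/Z grid coordinates using a fixed tile size.
; SwitchTile reads that cell's tile index, derives a TileTypes entry through modulo arithmetic, and writes it back, printing debug values.
; The construction script assigns the Map asset.
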(event `SwitchTile`
  (bind (_returnvalue _returnvalue2) (`self.GetTilePos`))
  (bind _tileindex (`self.GetTileType`))
  (`PaperTileMapComponent.MakeTileMapEditable` (`self.PaperTileMap`))
  (set `self.Tile_Num` _tileindex)
  (`KismetSystemLibrary.PrintString` (`KismetStringLibrary.Conv_IntToString` _tileindex))
  (set `self.Tile_Num` (mod (+ -7 (`self.Tile_Num`)) 4))
  (`PaperTileMapComponent.SetTile` (`self.PaperTileMap`) _returnvalue _returnvalue2 0 (`|GetArrayItem` (`self.TileTypes`) (- (`self.Tile_Num`) 8)))
  (`KismetSystemLibrary.PrintString` (`KismetStringLibrary.Conv_IntToString` (`self.Tile_Num`))))

(fn `CheckTilePos`)

(fn `PrintTilePos`
  (bind (_returnvalue _returnvalue2) (`self.GetTilePos`))
  (`KismetSystemLibrary.PrintString` (`KismetStringLibrary.Conv_VectorToString` (`KismetMathLibrary.MakeVector` (`KismetMathLibrary.Conv_IntToDouble` _returnvalue) 0.0 (`KismetMathLibrary.Conv_IntToDouble` _returnvalue2)))))

(fn `UserConstructionScript`
  (`PaperTileMapComponent.SetTileMap` (`self.PaperTileMap`) (`self.Map`)))