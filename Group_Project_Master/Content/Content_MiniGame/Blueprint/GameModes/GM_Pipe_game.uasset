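; Game mode for the pipe minigame that sets up mouse play and returns to the PLVL_World level on completion.
; BeginPlay shows the cursor on the PipeGameController, and Tick reapplies game-only input mode every frame.
; LevelCompleted calls a fade out and opens the world level.
; MakeHud creates, stores and displays the Mini_HUD_2 widget, but nothing in this Blueprint calls it.
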(event `self.ReceiveBeginPlay`
  (bind _returnvalue (`GameplayStatics.GetPlayerController` 0))
  (bind _aspipe_game_controller (cast `/Game/Content_MiniGame/Blueprint/PipeGameController` _returnvalue))
  (set `PlayerController.bShowMouseCursor` true _aspipe_game_controller)
  (`WidgetBlueprintLibrary.SetInputMode_GameOnly` _returnvalue :!label _label))

(event `self.ReceiveTick`
  (params (DeltaSeconds :type "Float (single-precision)"))
  (goto _label))

(event `LevelCompleted`
  (`/Game/Blueprints/BP_CameraFade.FadeOut` 0.0)
  (`GameplayStatics.OpenLevel` "PLVL_World"))

(fn `Make Hud`
  (bind _returnvalue (`|CreateWidget` "/Game/Content_MiniGame/UI/Mini_HUD_2.Mini_HUD_2_C"))
  (set `self.HudRef2` _returnvalue)
  (`UserWidget.AddToPlayerScreen` _returnvalue 0))

(fn `UserConstructionScript`)