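; Test game mode for mini-game levels that tracks objectives and score, and returns to the world map level on completion.
; Objectives register into a counter, but the clear check on each cleared objective compares current score to target score.
; A match fires the level-clear event, bound at BeginPlay, which fades out, removes the HUD and opens PLVL_World.
; Helper functions create the HUD and decrement the objective count.
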(event `/Game/Content_MiniGame/Blueprint/BPI_NodeCleared.registerObjective`
  ;[1 1 1] MiniGame_Initiation
  (`self.countObjective`))

(event `/Game/Content_MiniGame/Blueprint/BPI_NodeCleared.objectiveCleared`
  ;[1 1 1] MiniGame_Initiation
  (bind _cleared (`self.isLevelCleared`))
  (if _cleared
    (`KismetSystemLibrary.PrintString` "Level Cleared")
    (`KismetSystemLibrary.Delay` 0.5)
    (`self.LevelClearEvent`)
    (else
      (`KismetSystemLibrary.PrintString` "Not cleared yet."))))

(event `self.ReceiveBeginPlay`
  (add `self.LevelClearEvent` (delegate `LevelEnd`))
  (`self.ResetPlayerScore`))

(event `LevelEnd`
  ;[1 1 1] Events for what happens when a mini game level is finished
  (`self.HandleLevelEnd`))

(event `HandleLevelEnd`
  ;[1 1 1] Events for what happens when a mini game level is finished
  (`/Game/Content_MiniGame/Blueprint/BP_CameraFades.FadeOut` 1.0)
  (`KismetSystemLibrary.Delay` 1.0)
  (`Widget.RemoveFromParent` (`self.HUDRef`)) ; Remove UI
  (`GameplayStatics.OpenLevel` "PLVL_World"))

(fn `countObjective`
  ;[1 1 1] Set the number of objectives in a level.
  (bind _output_get (set `self.numObjective` (`self.numObjective`)))
  (`/Engine/EditorBlueprintResources/StandardMacros.IncrementInt` _output_get))

(fn `isLevelCleared`
  (returns (cleared :type Boolean))
  (return (== (`self.TargetScore`) (`self.CurrentScore`))))

(fn `MakeHUD`
  (bind _returnvalue (`|CreateWidget` "/Game/Content_MiniGame/UI/Mini_HUD.Mini_HUD_C"))
  (set `self.HUDRef` _returnvalue)
  (`UserWidget.AddToPlayerScreen` _returnvalue 0))

(fn `ResetPlayerScore`
  (set `self.CurrentScore` 0))

(fn `updateNumObjective`
  (`/Engine/EditorBlueprintResources/StandardMacros.DecrementInt` (`self.numObjective`)))

(fn `UserConstructionScript`)