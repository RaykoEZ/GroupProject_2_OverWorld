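; Player-side physics interaction Blueprint that lets objects be picked up, carried and thrown with the mouse.
; Left mouse line-traces within a wheel-adjustable pickup distance and grabs sufficiently light hits through a runtime-added Physics Handle, ignoring Pawn collision.
; Tick holds the object along the control rotation at its grab-time distance.
; Release drops it, adds a forward impulse if Q is held, and sets its WorldStatic response to Ignore.
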(event `self.ReceiveTick`
  (params (DeltaSeconds :type "Float (single-precision)"))
  ;[1 1 1] Set pickup object location
  (if (`self.Physics Handle Active`)
    (set `self.Handle Location` (+ (`self.K2_GetActorLocation`) (* (`KismetMathLibrary.GetForwardVector` (`self.GetControlRotation`)) (`self.Other item Location`))))
    (`PhysicsHandleComponent.SetTargetLocationAndRotation` (`self.PhysicsHandle`) (`self.Handle Location`) (`self.GetControlRotation`))))

(event `Key|MouseScrollUp`
  (params (Key :type "Key Structure" :default "AnyKey"))
  ;[1 1 1] Adjust pickup distance
  (:`Pressed`
    (set `self.Pick Up Distance` (+ (`self.Pick Up Distance`) 25.0))))

(event `Key|MouseScrollDown`
  (params (Key :type "Key Structure" :default "AnyKey"))
  ;[1 1 1] Adjust pickup distance
  (:`Pressed`
    (set `self.Pick Up Distance` (+ (`self.Pick Up Distance`) -25.0))))

(event `Key|Q`
  (params (Key :type "Key Structure" :default "AnyKey"))
  ;[1 1 1] Throw Object if Q is Held
  (:`Pressed`
    (set `self.Is Held?` true))
  (:`Released`
    (set `self.Is Held?` false)))

(event `InputAction|Left Mouse`
  (params (Key :type "Key Structure" :default "AnyKey"))
  (bind _bp_fpchar (`self.BP_FPChar`))
  (bind _returnvalue (`SceneComponent.GetForwardVector` _bp_fpchar))
  ;[1 1 1] Set Physics Handle active
  (:`Pressed`
    (set `self.Physics Handle Active` true)
    ;[1 1 1] Line Trace for Physics Objects
    (bind (_outhit _returnvalue_2) (`KismetSystemLibrary.LineTraceSingleForObjects` _returnvalue (+ _returnvalue (* (`SceneComponent.K2_GetComponentLocation` _bp_fpchar) (`self.Pick Up Distance`))) (`|MakeArray` (`self.Physics Object Types`))))
    (bind (_bblockinghit _binitialoverlap _time _location _impactpoint _normal _impactnormal _physmat _hitactor _hitcomponent _hitbonename) (`GameplayStatics.BreakHitResult` _outhit))
    ;[1 1 1] Get Other Object Location
    (set `self.Other Item Location` (`KismetMathLibrary.VSize` (- (`self.K2_GetActorLocation`) _location)))
    (set `self.Other Item Rotation` (`self.K2_GetActorRotation`))
    ;[1 1 1] Hit Conditions
    (if _returnvalue_2
      (if (< (`PrimitiveComponent.GetMass` _hitcomponent) 500.0)
        ;[1 1 1] Add & Grab Physics Handle
        (`AddComponent|NODE_AddPhysicsHandleComponent-0`)
        (set `self.PhysicsHandle` null)
        (set `self.Physics Body` _hitcomponent)
        (`PhysicsHandleComponent.GrabComponentAtLocation` (`self.PhysicsHandle`) _hitcomponent _hitbonename _location)
        (`PrimitiveComponent.SetCollisionResponseToChannel` _hitcomponent "ECC_Pawn" "ECR_Ignore"))))
  (:`Released`
    (set `self.Physics Handle Active` false)
    (`PhysicsHandleComponent.ReleaseComponent` (`self.PhysicsHandle`))
    ;[1 1 1] Throw Object if Q is Held
    (if (`self.Is Held?`)
      (`PrimitiveComponent.AddImpulse` _hitcomponent (* (`SceneComponent.GetForwardVector` (`self.BP_FPChar`)) 5000) "None" false))
    (`PrimitiveComponent.SetCollisionResponseToChannel` _hitcomponent "ECC_WorldStatic" "ECR_Ignore")))

(fn `UserConstructionScript`)