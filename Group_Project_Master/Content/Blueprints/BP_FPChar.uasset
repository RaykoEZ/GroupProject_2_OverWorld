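; BP_FPChar is a first-person character with movement, mouse look, toggle crouch on Left Ctrl and a HUD created at BeginPlay.
; Left click line-traces from the camera for physics objects and activates per-tick updates of a physics handle target ahead of the view.
; The logic that creates the handle and grabs objects under a mass limit is disconnected, so pickup never completes.
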(event `Key|LeftControl`
  (params (Key :type "Key Structure" :default "AnyKey"))
  ;[1 1 1] Crouch
  (:`Pressed`
    (`/Engine/EditorBlueprintResources/StandardMacros.FlipFlop`
      (:`A`
        (`self.Crouch`))
      (:`B`
        (`self.UnCrouch`)))))

(event `InputAxis|MoveForward`
  (params (AxisValue :type "Float (single-precision)"))
  ;[1 1 1] Moving Forwards/Backwards
  (`self.AddMovementInput` (`KismetMathLibrary.GetForwardVector` (`self.GetControlRotation`)) AxisValue))

(event `self.ReceiveBeginPlay`
  (`self.CreateHUD`))

(event `InputAxis|MoveRight`
  (params (AxisValue :type "Float (single-precision)"))
  ;[1 1 1] Move Left/Right
  (`self.AddMovementInput` (`KismetMathLibrary.GetRightVector` (`self.GetControlRotation`)) AxisValue))

(event `InputAxis|Turn`
  (params (AxisValue :type "Float (single-precision)"))
  ;[1 1 1] Rotating Character
  (`self.AddControllerYawInput` AxisValue))

(event `InputAxis|LookUp`
  (params (AxisValue :type "Float (single-precision)"))
  ;[1 1 1] Rotating Character
  (`self.AddControllerPitchInput` AxisValue))

(event `Key|LeftMouseButton`
  (params (Key :type "Key Structure" :default "AnyKey"))
  (bind _firstpersoncamera (`self.FirstPersonCamera`))
  (bind _returnvalue (`SceneComponent.K2_GetComponentLocation` _firstpersoncamera))
  (:`Pressed`
    (set `self.Physics Handle active` true)
    (bind (_outhit _returnvalue_2) (`KismetSystemLibrary.LineTraceSingleForObjects` _returnvalue (+ _returnvalue (* (`SceneComponent.GetForwardVector` _firstpersoncamera) 350.0)) (`self.Physics Object Type`)))))

(event `self.ReceiveTick`
  (params (DeltaSeconds :type "Float (single-precision)"))
  (if (`self.Physics Handle active`)
    (set `self.Handle Location` (+ (+ (`self.K2_GetActorLocation`) (* (`KismetMathLibrary.GetForwardVector` (`self.GetControlRotation`)) (`self.Object Location`))) (0.0 0.0 50.0)))
    (`PhysicsHandleComponent.SetTargetLocationAndRotation` (`self.Physics handle`) (`self.Handle Location`) (`self.K2_GetActorRotation`))))

(fn `CreateHUD`
  (bind _returnvalue (`|CreateWidget` "/Game/UI/BP_HUD.BP_HUD_C"))
  (`UserWidget.AddToPlayerScreen` _returnvalue 0))

(fn `UserConstructionScript`)