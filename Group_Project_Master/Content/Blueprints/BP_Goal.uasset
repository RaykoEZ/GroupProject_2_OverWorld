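; BP_Goal is an interactable trigger that sends the player from the first-person world into the minigame level named by MiniGameName.
; Overlapping Box_Trigger enables E input and shows the character HUD's interact prompt, and leaving reverses both.
; Pressing E stores the player's transform in the BP_GlobalData game instance, hides the prompt, fades out and opens the level after a short delay.
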(event `self.ReceiveBeginPlay`
  ;[1 1 1] iNITIALIZATION
  (bind _asbp_fpcharacter (cast `/Game/Blueprints/BP_FPCharacter` (`GameplayStatics.GetPlayerCharacter` 0)))
  (set `self.CharHUD` (`/Game/Blueprints/BP_FPCharacter.HUDRef` _asbp_fpcharacter)))

(event `self.Box_Trigger.OnComponentBeginOverlap`
  (params (OverlappedComponent :type "PrimitiveComponent Object Reference") (OtherActor :type "Actor Object Reference") (OtherComp :type "PrimitiveComponent Object Reference") (OtherBodyIndex :type Integer) (bFromSweep :type Boolean) (SweepResult :type "HitResult Structure (by ref)"))
  (bind _charhud (`self.CharHUD`))
  ;[1 1 1] Overlap events
  (`/Engine/EditorBlueprintResources/StandardMacros.IsValid` _charhud
    (:`Is Valid`
      (`self.EnableInput` (`GameplayStatics.GetPlayerController` 0))
      (`/Game/UI/BP_FP_HUD.InteractPopUp` _charhud))))

(event `self.Box_Trigger.OnComponentEndOverlap`
  (params (OverlappedComponent :type "PrimitiveComponent Object Reference") (OtherActor :type "Actor Object Reference") (OtherComp :type "PrimitiveComponent Object Reference") (OtherBodyIndex :type Integer))
  ;[1 1 1] Overlap events
  (`self.DisableInput` (`GameplayStatics.GetPlayerController` 0))
  (`/Game/UI/BP_FP_HUD.InteractPopOff` (`self.CharHUD`)))

(event `Key|E`
  (params (Key :type "Key Structure" :default "AnyKey"))
  ;[1 1 1] Event for interaction
  (:`Pressed`
    (bind _asbp_global_data (cast `/Game/Blueprints/BP_GlobalData` (`GameplayStatics.GetGameInstance`)))
    (bind _asbp_fpcharacter (cast `/Game/Blueprints/BP_FPCharacter` (`GameplayStatics.GetPlayerCharacter` 0)))
    (set `/Game/Blueprints/BP_GlobalData.FP_PlayerTransform` (`self.GetTransform` _asbp_fpcharacter) _asbp_global_data)
    (`/Game/UI/BP_FP_HUD.InteractPopOff` (`self.CharHUD`))
    (`/Game/Content_MiniGame/Blueprint/BP_CameraFades.FadeOut` 1.0)
    (`KismetSystemLibrary.Delay` 1.0)
    (`GameplayStatics.OpenLevel` (`self.MiniGameName`)) ; Open MiniGame level
  ))

(fn `UserConstructionScript`)