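; BP_PanelTrigger is an interactable button panel that calls a lift's door update for its configured floor.
; On BeginPlay it finds the first valid BP_Lift among actors tagged "Lift" and keeps a reference to it.
; InteractEvent passes ToFloor to that lift's CallUpdateDoor, and the construction script applies the configurable ButtonMesh to the button component.
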(event `self.ReceiveBeginPlay`
  ;[1 1 1] Initialize
  (bind _outactors (`GameplayStatics.GetAllActorsWithTag` "Lift"))
  (for _array_element _outactors
    (bind _asbp_lift (cast `/Game/Blueprints/BP_Lift` _array_element))
    (`/Engine/EditorBlueprintResources/StandardMacros.IsValid` _asbp_lift
      (:`Is Valid`
        (set `self.liftRef` _asbp_lift)
        (`KismetSystemLibrary.PrintString` "found lift")
        (break)))))

(event `/Game/Blueprints/BPI_Interactive.InteractEvent`
  ;[1 1 1] Event for opening doors
  (`/Game/Blueprints/BP_Lift.updateDoor` (`self.liftRef`) (`self.toFloor`)))

(fn `UserConstructionScript`
  (`StaticMeshComponent.SetStaticMesh` (`self.button1`) (`self.buttonMesh`)))