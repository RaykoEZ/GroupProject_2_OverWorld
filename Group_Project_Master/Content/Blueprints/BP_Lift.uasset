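; BP_Lift is an elevator actor that changes floors when its bound UpdateDoorState event receives a target floor.
; It validates the floor, closes the door, shifts the actor by a timeline vector scaled by the floor offset, then reopens, sequenced with fixed delays.
; Timelines lerp the door, while the lift jumps only when its timeline finishes and CheckOffset steps CurrentLevel by one.
; FinishEvent then notifies BP_FPCharacter that the interaction is over.
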(event `self.ReceiveBeginPlay`
  ;[1 1 1] Initializing
  (add `self.updateDoor` (delegate `updateDoorState`))
  (set `self.InitialDoorLocation` (`SceneComponent.RelativeLocation` (`self.SM_Door`)))
  (`KismetSystemLibrary.Delay` 1.0)
  (`self.DoorOpening`)
  (`KismetSystemLibrary.Delay` 3.0)
  (`self.FinishEvent`))

(event `updateDoorState` :!signature `self.updateDoor`
  (params (toFloor :type Integer))
  (bind _currentlevel (`self.currentLevel`))
  ;[1 1 1] Door and liift event here
  (if (and (<= toFloor (`self.maxLevel`)) (!= _currentlevel toFloor))
    (if (`self.DoorOpen`)
      (`self.DoorClosing`))
    (`KismetSystemLibrary.Delay` 3.0)
    (`self.Descend` (- toFloor _currentlevel))
    (`KismetSystemLibrary.Delay` 2.0)
    (`self.DoorOpening`)
    (`KismetSystemLibrary.Delay` 3.0)
    (`self.FinishEvent`)
    (else
      (`KismetSystemLibrary.PrintString` "Bad Floor")
      (`self.FinishEvent`))))

(event `Descend`
  (params (offset :type Integer))
  ;[1 1 1] Door and liift event here
  (bind (_direction _newtrack_0) (`Timeline|GoDown` :!via `PlayFromStart`)
    (:`Finished`
      (`self.K2_SetActorRelativeLocation` (- (`self.K2_GetActorLocation`) (* _newtrack_0 offset)))
      (`self.CheckOffset` offset))))

(event `DoorOpening`
  ;[1 1 1] Door and liift event here
  (bind (_direction _doormove) (`Timeline|OpenDoor` :!via `PlayFromStart`) ; Animation for open/closing doors
    (:`Update`
      (set `self.DoorOpen` true)
      (`SceneComponent.K2_SetRelativeLocation` (`self.SM_Door`) (`KismetMathLibrary.VLerp` (`self.InitialDoorLocation`) (`self.endDoorLocation`) (.x _doormove)) false false))))

(event `DoorClosing`
  ;[1 1 1] Door and liift event here
  (bind (_direction _doormove) (`Timeline|Close` :!via `ReverseFromEnd`) ; Animation for open/closing doors
    (:`Update`
      (set `self.DoorOpen` false)
      (`SceneComponent.K2_SetRelativeLocation` (`self.SM_Door`) (`KismetMathLibrary.VLerp` (`self.InitialDoorLocation`) (`self.endDoorLocation`) (.x _doormove)) false false))))

(fn `UserConstructionScript`)