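; BP_Goal is a level goal actor that reveals a LevelComplete component while something overlaps its trigger box.
; Box_Trigger's begin and end overlap events show and hide that component without checking what overlaps or propagating to children.
; The construction script applies the BoundMesh variable to the Mesh component, so the goal's static mesh follows that variable.
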(event `self.Box_Trigger.OnComponentBeginOverlap`
  (params (OverlappedComponent :type "PrimitiveComponent Object Reference") (OtherActor :type "Actor Object Reference") (OtherComp :type "PrimitiveComponent Object Reference") (OtherBodyIndex :type Integer) (bFromSweep :type Boolean) (SweepResult :type "HitResult Structure (by ref)"))
  (`SceneComponent.SetVisibility` (`self.LevelComplete`) true false))

(event `self.Box_Trigger.OnComponentEndOverlap`
  (params (OverlappedComponent :type "PrimitiveComponent Object Reference") (OtherActor :type "Actor Object Reference") (OtherComp :type "PrimitiveComponent Object Reference") (OtherBodyIndex :type Integer))
  (`SceneComponent.SetVisibility` (`self.LevelComplete`) false false))

(fn `UserConstructionScript`
  (`StaticMeshComponent.SetStaticMesh` (`self.Mesh`) (`self.BoundMesh`)))